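; Interactable switch that turns four disco lights on and off.
; A Box overlap sets a PlayerInHitBox flag, toggles a point light and text prompt, and prints a debug message on enter and exit.
; The Interaction event, gated by that flag, flips DiscoOn and calls DiscoOn or DiscoOff on the four referenced lights.
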(event `self.Interaction`
  (if (`self.PlayerInHitBox`)
    (if (`self.DiscoOn`)
      (`|ExecutionSequence`
        (:`then_0`
          (`/Game/Arcady_TPS/Blueprints/Obstacles/SmallLightSource.DiscoOff` (`self.Light1`)))
        (:`then_1`
          (`/Game/Arcady_TPS/Blueprints/Obstacles/SmallLightSource.DiscoOff` (`self.Light2`)))
        (:`then_2`
          (`/Game/Arcady_TPS/Blueprints/Obstacles/SmallLightSource.DiscoOff` (`self.Light3`)))
        (:`then_3`
          (`/Game/Arcady_TPS/Blueprints/Obstacles/SmallLightSource.DiscoOff` (`self.Light4`)))
        (:`then_4`
          (set `self.DiscoOn` false)))
      (else
        (`|ExecutionSequence`
          (:`then_0`
            (`/Game/Arcady_TPS/Blueprints/Obstacles/SmallLightSource.DiscoOn` (`self.Light1`)))
          (:`then_1`
            (`/Game/Arcady_TPS/Blueprints/Obstacles/SmallLightSource.DiscoOn` (`self.Light2`)))
          (:`then_2`
            (`/Game/Arcady_TPS/Blueprints/Obstacles/SmallLightSource.DiscoOn` (`self.Light3`)))
          (:`then_3`
            (`/Game/Arcady_TPS/Blueprints/Obstacles/SmallLightSource.DiscoOn` (`self.Light4`)))
          (:`then_4`
            (set `self.DiscoOn` true)))))))

(event `self.Box.OnComponentBeginOverlap`
  (params (OverlappedComponent :type "PrimitiveComponent Object Reference") (OtherActor :type "Actor Object Reference") (OtherComp :type "PrimitiveComponent Object Reference") (OtherBodyIndex :type Integer) (bFromSweep :type Boolean) (SweepResult :type "HitResult Structure (by ref)"))
  (`|ExecutionSequence`
    (:`then_0`
      (set `self.PlayerInHitBox` true)
      (`KismetSystemLibrary.PrintString` "Player In Hit Box" true true (struct :`G` 0.66 :`B` 1.0 :`A` 1.0) 3.0))
    (:`then_1`
      (`SceneComponent.SetVisibility` (`self.Point Light`) true false))
    (:`then_2`
      (`SceneComponent.SetVisibility` (`self.TextRender`) true false))))

(event `self.Box.OnComponentEndOverlap`
  (params (OverlappedComponent :type "PrimitiveComponent Object Reference") (OtherActor :type "Actor Object Reference") (OtherComp :type "PrimitiveComponent Object Reference") (OtherBodyIndex :type Integer))
  (`|ExecutionSequence`
    (:`then_0`
      (set `self.PlayerInHitBox` false)
      (`KismetSystemLibrary.PrintString` "Player Out Hit Box" true true (struct :`G` 0.66 :`B` 1.0 :`A` 1.0) 3.0))
    (:`then_1`
      (`SceneComponent.SetVisibility` (`self.Point Light`) false false))
    (:`then_2`
      (`SceneComponent.SetVisibility` (`self.TextRender`) false false))))

(fn `UserConstructionScript`
  (`parent.UserConstructionScript`))