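; LightSource is an obstacle-folder Blueprint that makes a lamp flicker with random colors and brightness.
; From BeginPlay, a self-repeating event waits a random delay between MinDelay and MaxDelay, then calls RandomLights and loops.
; RandomLights gives the PointLight a fully random RGB color and an intensity picked between MinIntensity and MaxIntensity.
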(event `Repeat`
  ;[1 1 1] Мигание света ламп
  (`KismetSystemLibrary.Delay` (`KismetMathLibrary.RandomFloatInRange` (`self.MinDelay`) (`self.MaxDelay`)) :!label _label)
  (`self.RandomLights`)
  (`self.Repeat`))

(event `self.ReceiveBeginPlay`
  ;[1 1 1] Мигание света ламп
  (goto _label))

(fn `RandomLights`
  (bind _pointlight (`self.PointLight`))
  ;[1 1 1] Выбор нового цвета и уровня интенсивности источника света
  (`LightComponent.SetLightColor` _pointlight (`KismetMathLibrary.MakeColor` (`KismetMathLibrary.RandomFloatInRange` 0.0 1.0) (`KismetMathLibrary.RandomFloatInRange` 0.0 1.0) (`KismetMathLibrary.RandomFloatInRange` 0.0 1.0)) true)
  (`LightComponent.SetIntensity` _pointlight (`KismetMathLibrary.RandomFloatInRange` (`self.MinIntensity`) (`self.MaxIntensity`))))

(fn `UserConstructionScript`)