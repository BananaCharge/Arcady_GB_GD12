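; SmallLightSource is a light Blueprint with a switchable disco mode for its PointLight.
; DiscoOn sets the Disco flag and enters the Repeat loop, which waits a random MinDelay–MaxDelay interval, calls RandomLights, then re-triggers itself while the flag holds.
; DiscoOff only clears the flag, so the loop restores a fixed warm color and intensity after its next pending delay and RandomLights call.
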(event `self.Repeat`
  (bind _pointlight (`self.PointLight`))
  ;[1 1 1] Режим дискотеки
  (`KismetSystemLibrary.Delay` (`KismetMathLibrary.RandomFloatInRange` (`self.MinDelay`) (`self.MaxDelay`)) :!label _label)
  (`self.RandomLights`)
  (if (`self.Disco`)
    (`self.Repeat`)
    (else
      ;[1 1 1] Выключение режима дискотеки
      (`LightComponent.SetLightColor` _pointlight (struct :`R` 0.807292 :`G` 0.693804 :`B` 0.467053 :`A` 1.0) true)
      (`LightComponent.SetIntensity` _pointlight 3000.0))))

(event `DiscoOn`
  ;[1 1 1] Режим дискотеки
  (`|ExecutionSequence`
    (:`then_0`
      (set `self.Disco` true))
    (:`then_1`
      (goto _label))))

(event `DiscoOff`
  ;[1 1 1] Выключение режима дискотеки
  (set `self.Disco` false))

(fn `UserConstructionScript`
  (`parent.UserConstructionScript`))