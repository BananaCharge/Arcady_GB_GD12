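; LightSource is a Blueprint that makes its point light flicker through random colors and brightness levels.
; From BeginPlay it waits a random delay between configurable minimum and maximum values, then calls RandomLights and loops through the Repeat event.
; RandomLights gives the PointLight component a fully random RGB color and a random intensity within a configurable range.
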(event `Repeat`
  (`KismetSystemLibrary.Delay` (`KismetMathLibrary.RandomFloatInRange` (`self.MinDelay`) (`self.MaxDelay`)) :!label _label)
  (`self.RandomLights`)
  (`self.Repeat`))

(event `self.ReceiveBeginPlay`
  (goto _label))

(fn `RandomLights`
  (bind _pointlight (`self.PointLight`))
  (`LightComponent.SetLightColor` _pointlight (`KismetMathLibrary.MakeColor` (`KismetMathLibrary.RandomFloatInRange` 0.0 1.0) (`KismetMathLibrary.RandomFloatInRange` 0.0 1.0) (`KismetMathLibrary.RandomFloatInRange` 0.0 1.0)) true)
  (`LightComponent.SetIntensity` _pointlight (`KismetMathLibrary.RandomFloatInRange` (`self.MinIntensity`) (`self.MaxIntensity`))))

(fn `UserConstructionScript`)