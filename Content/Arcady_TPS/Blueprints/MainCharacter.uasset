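; Third-person shooter player character handling movement, jumping, sprinting, interaction and gun pickup.
; Camera look input only applies while the CamRotation action is held, and sprint swaps max walk speed.
; Capsule overlaps track the current Interractable and Gun, which the Interact input triggers or picks up.
; Picking up a gun disables its physics, snaps it to the Scene component and drops the equipped one with physics re-enabled.
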(event `self.CapsuleComponent.OnComponentBeginOverlap`
  (params (OverlappedComponent :type "PrimitiveComponent Object Reference") (OtherActor :type "Actor Object Reference") (OtherComp :type "PrimitiveComponent Object Reference") (OtherBodyIndex :type Integer) (bFromSweep :type Boolean) (SweepResult :type "HitResult Structure (by ref)"))
  (`|ExecutionSequence`
    (:`then_0`
      (bind _asinterractable (cast `/Game/Arcady_TPS/Blueprints/Obstacles/Interractable` OtherActor))
      (set `self.InteractableObj` _asinterractable))
    (:`then_1`
      (bind _asgun (cast `/Game/Arcady_TPS/Blueprints/Weapon/Gun` OtherActor))
      (set `self.InteractableGun` _asgun))))

(event `InputAxis|MoveForward`
  (params (AxisValue :type "Float (single-precision)"))
  ;[0.2344 0.2344 0.2344] Walking Controller
  (`self.AddMovementInput` (`self.GetActorForwardVector`) AxisValue))

(event `InputAxis|LookUp`
  (params (AxisValue :type "Float (single-precision)"))
  ;[0.1615 0.1615 0.1615] Rotation Controller
  (if (`self.CamCanRotate`)
    (`self.AddControllerPitchInput` AxisValue)))

(event `InputAxis|Turn`
  (params (AxisValue :type "Float (single-precision)"))
  ;[0.1615 0.1615 0.1615] Rotation Controller
  (if (`self.CamCanRotate`)
    (`self.AddControllerYawInput` AxisValue)))

(event `InputAxis|MoveRight`
  (params (AxisValue :type "Float (single-precision)"))
  ;[0.2344 0.2344 0.2344] Walking Controller
  (`self.AddMovementInput` (`self.GetActorRightVector`) AxisValue))

(event `self.CapsuleComponent.OnComponentEndOverlap`
  (params (OverlappedComponent :type "PrimitiveComponent Object Reference") (OtherActor :type "Actor Object Reference") (OtherComp :type "PrimitiveComponent Object Reference") (OtherBodyIndex :type Integer))
  (`|ExecutionSequence`
    (:`then_0`
      (bind _asinterractable (cast `/Game/Arcady_TPS/Blueprints/Obstacles/Interractable` OtherActor))
      (if (== _asinterractable (`self.InteractableObj`))
        (set `self.InteractableObj` null)))
    (:`then_1`
      (bind _asgun (cast `/Game/Arcady_TPS/Blueprints/Weapon/Gun` OtherActor))
      (if (== _asgun (`self.InteractableGun`))
        (set `self.InteractableGun` null)))))

(event `InputAction|CamRotation`
  (params (Key :type "Key Structure"))
  ;[0.1615 0.1615 0.1615] Rotation Controller
  (:`Pressed`
    (set `self.CamCanRotate` true)
    (`KismetSystemLibrary.PrintString` "Camera Released" true true (struct :`G` 0.66 :`B` 1.0 :`A` 1.0) 1.0))
  (:`Released`
    (set `self.CamCanRotate` false)
    (`KismetSystemLibrary.PrintString` "Camera Locked" true true (struct :`G` 0.66 :`B` 1.0 :`A` 1.0) 1.0)))

(event `InputAction|Sprint`
  (params (Key :type "Key Structure"))
  (bind _charactermovement (`self.CharacterMovement`))
  ;[0.2344 0.2344 0.2344] Walking Controller
  (:`Pressed`
    (set `CharacterMovementComponent.MaxWalkSpeed` 1500.0 _charactermovement)
    (`KismetSystemLibrary.PrintString` "Sprint On"))
  (:`Released`
    (set `CharacterMovementComponent.MaxWalkSpeed` 600.0 _charactermovement)
    (`KismetSystemLibrary.PrintString` "Sprint Off")))

(event `InputAction|Interact`
  (params (Key :type "Key Structure"))
  (bind _interactableobj (`self.InteractableObj`))
  (:`Pressed`
    (`|ExecutionSequence`
      (:`then_0`
        (if (`KismetSystemLibrary.IsValid` _interactableobj)
          (`/Game/Arcady_TPS/Blueprints/Obstacles/Interractable.Interaction` _interactableobj)))
      (:`then_1`
        (if (`KismetSystemLibrary.IsValid` (`self.InteractableGun`))
          (`self.PickUpNewGun`))))))

(event `InputAction|Jump`
  (params (Key :type "Key Structure"))
  ;[0.2344 0.2344 0.2344] Walking Controller
  (:`Pressed`
    (`self.Jump`)))

(fn `DropGun`
  (bind _gunequiped (`self.GunEquiped`))
  (if (`KismetSystemLibrary.IsValid` (`self.GunEquiped`))
    (`self.K2_DetachFromActor` _gunequiped "KeepWorld" "KeepWorld" "KeepWorld")
    (`PrimitiveComponent.SetSimulatePhysics` (`/Game/Arcady_TPS/Blueprints/Weapon/Gun.StaticMesh` _gunequiped) true)
    (set `self.GunEquiped` null)))

(fn `PickUpNewGun`
  (bind _interactablegun (`self.InteractableGun`))
  (if (!= (`self.InteractableGun`) (`self.GunEquiped`))
    (`PrimitiveComponent.SetSimulatePhysics` (`/Game/Arcady_TPS/Blueprints/Weapon/Gun.StaticMesh` _interactablegun) false)
    (`self.K2_AttachToComponent` _interactablegun (`self.Scene`) "None" "SnapToTarget" "SnapToTarget" "KeepWorld" true)
    (`self.DropGun`)
    (set `self.GunEquiped` (`self.InteractableGun`))
    (set `self.InteractableGun` null)))

(fn `UserConstructionScript`)